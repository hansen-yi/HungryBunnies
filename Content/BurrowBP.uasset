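; Burrow actor that can be covered over, swapping its open burrow mesh for a covered one.
; Its Cover function hides the Burrow component, shows BurrowCovered, and removes the actor's location from the Burrows collection on GlobalBP.
; When that removal succeeds, it decrements the Farmer's ShovelUses, so only a still-registered burrow costs a shovel use.
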(event EventBeginPlay)

(event Collision|EventActorBeginOverlap
  (params (OtherActor :type Actor%20Object%20Reference)))

(event EventTick
  (params (DeltaSeconds :type Float%20%28single-precision%29)))

(fn ConstructionScript)

(fn Cover
  (Rendering|SetVisibility (Variables|Default|GetBurrow) false false)
  (Rendering|SetVisibility (Variables|Default|GetBurrowCovered) true false)
  (bind _outactors (Actor|GetAllActorsOfClass "/Game/GlobalBP.GlobalBP_C"))
  (bind _returnvalue (Utilities|Array|RemoveItem (Variables|/Game/GlobalBP.GlobalBP_C|GetBurrows (Utilities|Array|Get(acopy) _outactors)) (Transformation|GetActorLocation)))
  (if _returnvalue
    (bind _returnvalue_2 (Actor|GetActorOfClass "/Game/Farmer.Farmer_C"))
    (Math|Integer|DecrementInt (Variables|/Game/Farmer.Farmer_C|GetShovelUses _returnvalue_2))))