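; Tree actor Blueprint that displays one to three apples and hides them as its apple count drops.
; BeginPlay picks a random NumApples from 1 to 3 and shows that many of the three Apple components.
; Tick polls NumApples every frame and hides the apple just above the current count, so the visuals follow decrements one at a time.
; Nothing in this graph changes the count after BeginPlay.
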(event EventBeginPlay
  (bind _output_get (Variables|Default|SetNumApples (Math|Random|RandomIntegerinRange 1 3)))
  (for _index (range 1 _output_get)
    (if (== _index 1)
      (Rendering|SetVisibility (Variables|Default|GetApple1) true false)
      (elif (== _index 2)
        (Rendering|SetVisibility (Variables|Default|GetApple2) true false)
        (elif (== _index 3)
          (Rendering|SetVisibility (Variables|Default|GetApple3) true false))))))

(event Collision|EventActorBeginOverlap
  (params (OtherActor :type Actor%20Object%20Reference)))

(event EventTick
  (params (DeltaSeconds :type Float%20%28single-precision%29))
  (bind _numapples (Variables|Default|GetNumApples))
  (if (< _numapples 3)
    (if (== _numapples 2)
      (Rendering|SetVisibility (Variables|Default|GetApple3) false false)
      (elif (== _numapples 1)
        (Rendering|SetVisibility (Variables|Default|GetApple2) false false)
        (elif (== _numapples 0)
          (Rendering|SetVisibility (Variables|Default|GetApple1) false false))))))

(fn ConstructionScript)