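; Spawner actor that scatters trees with apples inside a box volume when play begins.
; For each tree it picks random points in the Container bounds and line-traces downward from high above against the configured object types.
; Hits outside narrow bands along the world X and Y axes spawn a randomly yawed TreeBP at Z zero, plus an AppleBP just above it.
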(event EventBeginPlay
  (bind _container (Variables|Default|GetContainer))
  (bind (_origin _boxextent) (Collision|GetComponentBounds _container))
  (bind _returnvalue (Math|Random|RandomPointinBoundingBox _origin _boxextent))
  (bind (_x _y _z) (Math|Vector|BreakVector _returnvalue))
  (bind _returnvalue_2 (+ _z 1e+05))
  (bind _returnvalue_3 (Math|Vector|MakeVector _x _y _returnvalue_2))
  (if (Class|KismetMathLibrary|EqualExactlyVectorVector (Variables|Default|GetScaleContainer) "0, 0, 0")
    (Variables|Default|SetScaleContainer "500.000000,500.000000,500.000000"))
  (Components|Box|SetBoxExtent (Variables|Default|GetContainer) (Variables|Default|GetScaleContainer) false)
  (for _index (range 0 (- (Variables|Default|GetTreeCount) 1))
    (bind (_outhit _returnvalue_4) (Collision|LineTraceForObjects _returnvalue_3 (+ _returnvalue_3 (* (* (Transformation|GetActorUpVector) "-1.000000,-1.000000,-1.000000") "150000.000000,150000.000000,150000.000000")) (Variables|Default|GetAttachToObjs) false 0 "None"))
    (if _returnvalue_4
      (if (and (> (Math|Float|Absolute(Float) (.X (Math|Vector|BreakVector (.ImpactPoint (Collision|BreakHitResult _outhit))))) 3e+01) (> (Math|Float|Absolute(Float) (.Y (Math|Vector|BreakVector (.ImpactPoint (Collision|BreakHitResult _outhit))))) 3e+01))
        (Game|SpawnActorfromClass "/Game/TreeBP.TreeBP_C" (Math|Transform|MakeTransform (Math|Vector|MakeVector (.X (Math|Vector|BreakVector (.ImpactPoint (Collision|BreakHitResult _outhit)))) (.Y (Math|Vector|BreakVector (.ImpactPoint (Collision|BreakHitResult _outhit)))) 0.0) (Math|Rotator|MakeRotator 0.0 0.0 (Math|Random|RandomFloatinRange 0.0 (Variables|Default|GetMaxRotation)))) "AdjustIfPossibleButAlwaysSpawn" 0 0)
        (Game|SpawnActorfromClass "/Game/AppleBP.AppleBP_C" (Math|Transform|MakeTransform (+ (Math|Vector|MakeVector (.X (Math|Vector|BreakVector (.ImpactPoint (Collision|BreakHitResult _outhit)))) (.Y (Math|Vector|BreakVector (.ImpactPoint (Collision|BreakHitResult _outhit)))) 0.0) (Math|Vector|MakeVector 0.0 0.0 9e+01))) "Undefined" 0 0)))))

(event Collision|EventActorBeginOverlap
  (params (OtherActor :type Actor%20Object%20Reference)))

(event EventTick
  (params (DeltaSeconds :type Float%20%28single-precision%29)))

(fn ConstructionScript)