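; GlobalBP is the game manager for a farmer-and-bunny apple game, tracking carried and basket apple counts.
; On BeginPlay it scatters burrows at random and binds to basket, farmer and burrow events.
; Tree hits add carried apples; reaching the basket banks them and stops bunny spawning, while leaving restarts a looping spawn timer at random burrows.
; Arriving bunnies take basket apples; covering any burrow removes the last-spawned burrow's location from the spawn list.
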(event Custom|IncreaseCurrentApples
  (Variables|Default|SetCurrentApples (+ (Variables|Default|GetCurrentApples) 1)))

(event Custom|DecreaseBasketApples
  (if (> (Variables|Default|GetBasketApples) 0)
    (Variables|Default|SetBasketApples (- (Variables|Default|GetBasketApples) 1))))

(event Custom|TransferApples
  (Variables|Default|SetBasketApples (+ (Variables|Default|GetCurrentApples) (Variables|Default|GetBasketApples)))
  (Variables|Default|SetCurrentApples 0)
  (Utilities|Time|ClearandInvalidateTimerbyHandle (Variables|Default|GetBunnyTimer)))

(event Custom|RemoveBurrow
  (Utilities|Array|RemoveItem (Variables|Default|GetBurrows) (Transformation|GetActorLocation (stale EventBeginPlay _returnvalue))))

(event Custom|SpawnBunny
  (bind _burrows (Variables|Default|GetBurrows))
  (if (not (== (Utilities|Array|Length _burrows) 0))
    (Game|SpawnActorfromClass "/Game/BunnyBP.BunnyBP_C" (Math|Conversions|ToTransform(Vector) (.OutItem (Utilities|Array|Random _burrows))) "Undefined" 0 0)))

(event Custom|RestartBunnyTimer
  (bind _returnvalue (Utilities|Time|SetTimerbyFunctionName 0 "SpawnBunny" 1.0 true))
  (Variables|Default|SetBunnyTimer _returnvalue))

(event EventBeginPlay
  (bind _outactors (Actor|GetAllActorsOfClass "/Game/BasketBP.BasketBP_C"))
  (EventDispatchers|BindEventtoFarmerLeft _outactors (delegate Custom|RestartBunnyTimer))
  (EventDispatchers|BindEventtoBunnyArrived _outactors (delegate Custom|DecreaseBasketApples))
  (EventDispatchers|BindEventtoFarmerArrived _outactors (delegate Custom|TransferApples))
  (bind _outactors_2 (Actor|GetAllActorsOfClass "/Game/Farmer.Farmer_C"))
  (EventDispatchers|BindEventtoHitTree _outactors_2 (delegate Custom|IncreaseCurrentApples))
  (for _index (range 1 20)
    (bind _returnvalue (Game|SpawnActorfromClass "/Game/BurrowBP.BurrowBP_C" (Math|Conversions|ToTransform(Vector) (Math|Vector|MakeVector (Math|Random|RandomFloatinRange -3e+02 3e+02) (Math|Random|RandomFloatinRange -3e+02 3e+02) 0.0)) "Undefined" 0 0))
    (Utilities|Array|Add (Variables|Default|GetBurrows) (Transformation|GetActorLocation _returnvalue))
    (EventDispatchers|BindEventtoCoveringBurrow _returnvalue (delegate Custom|RemoveBurrow))))

(event Collision|EventActorBeginOverlap
  (params (OtherActor :type Actor%20Object%20Reference)))

(event EventTick
  (params (DeltaSeconds :type Float%20%28single-precision%29)))

(fn ConstructionScript)