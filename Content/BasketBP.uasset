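; Apple basket actor that signals bunny and farmer visits and displays the shared apple count.
; Its collider overlaps fire BunnyArrived, FarmerArrived and FarmerLeft dispatchers based on the other actor's class.
; Every Tick it looks up GlobalBP and, while BasketApples is below 13, walks nested checks over twelve apple components.
; The checks show apples up to the count but hide only the next one, so multi-apple drops can leave higher apples visible.
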(event OnComponentBeginOverlap(BasketCollider)
  (params (OverlappedComponent :type Primitive%20Component%20Object%20Reference) (OtherActor :type Actor%20Object%20Reference) (OtherComp :type Primitive%20Component%20Object%20Reference) (OtherBodyIndex :type Integer) (bFromSweep :type Boolean) (SweepResult :type Hit%20Result%20Structure%20%28by%20ref%29))
  (Utilities|Casting|CastToBunnyBP OtherActor
    (:then
      (Default|CallBunnyArrived))
    (:CastFailed
      (Utilities|Casting|CastToFarmer OtherActor)
      (Default|CallFarmerArrived))))

(event OnComponentEndOverlap(BasketCollider)
  (params (OverlappedComponent :type Primitive%20Component%20Object%20Reference) (OtherActor :type Actor%20Object%20Reference) (OtherComp :type Primitive%20Component%20Object%20Reference) (OtherBodyIndex :type Integer))
  (Utilities|Casting|CastToFarmer OtherActor)
  (Default|CallFarmerLeft))

(event EventBeginPlay)

(event Collision|EventActorBeginOverlap
  (params (OtherActor :type Actor%20Object%20Reference)))

(event EventTick
  (params (DeltaSeconds :type Float%20%28single-precision%29))
  (bind _apple4 (Variables|Default|GetApple4))
  (bind _apple5 (Variables|Default|GetApple5))
  (bind _apple6 (Variables|Default|GetApple6))
  (bind _apple7 (Variables|Default|GetApple7))
  (bind _apple8 (Variables|Default|GetApple8))
  (bind _apple9 (Variables|Default|GetApple9))
  (bind _apple10 (Variables|Default|GetApple10))
  (bind _apple11 (Variables|Default|GetApple11))
  (bind _apple12 (Variables|Default|GetApple12))
  (bind _returnvalue (Actor|GetActorOfClass "/Game/GlobalBP.GlobalBP_C"))
  (if (< (Variables|/Script/HungryBunnies.Global|GetBasketApples _returnvalue) 13)
    (if (> (Variables|/Script/HungryBunnies.Global|GetBasketApples _returnvalue) 0)
      (Rendering|SetVisibility (Variables|Default|GetApple1) true false)
      (if (> (Variables|/Script/HungryBunnies.Global|GetBasketApples _returnvalue) 1)
        (Rendering|SetVisibility (Variables|Default|GetApple2) true false)
        (if (> (Variables|/Script/HungryBunnies.Global|GetBasketApples _returnvalue) 2)
          (Rendering|SetVisibility (Variables|Default|GetApple3) true false)
          (if (> (Variables|/Script/HungryBunnies.Global|GetBasketApples _returnvalue) 3)
            (Rendering|SetVisibility _apple4 true false)
            (if (> (Variables|/Script/HungryBunnies.Global|GetBasketApples _returnvalue) 4)
              (Rendering|SetVisibility _apple5 true false)
              (if (> (Variables|/Script/HungryBunnies.Global|GetBasketApples _returnvalue) 5)
                (Rendering|SetVisibility _apple6 true false)
                (if (> (Variables|/Script/HungryBunnies.Global|GetBasketApples _returnvalue) 6)
                  (Rendering|SetVisibility _apple7 true false)
                  (if (> (Variables|/Script/HungryBunnies.Global|GetBasketApples _returnvalue) 7)
                    (Rendering|SetVisibility _apple8 true false)
                    (if (> (Variables|/Script/HungryBunnies.Global|GetBasketApples _returnvalue) 8)
                      (Rendering|SetVisibility _apple9 true false)
                      (if (> (Variables|/Script/HungryBunnies.Global|GetBasketApples _returnvalue) 9)
                        (Rendering|SetVisibility _apple10 true false)
                        (if (> (Variables|/Script/HungryBunnies.Global|GetBasketApples _returnvalue) 10)
                          (Rendering|SetVisibility _apple11 true false)
                          (if (> (Variables|/Script/HungryBunnies.Global|GetBasketApples _returnvalue) 11)
                            (Rendering|SetVisibility _apple12 true false)
                            (else
                              (Rendering|SetVisibility _apple12 false false)))
                          (else
                            (Rendering|SetVisibility _apple11 false false)))
                        (else
                          (Rendering|SetVisibility _apple10 false false)))
                      (else
                        (Rendering|SetVisibility _apple9 false false)))
                    (else
                      (Rendering|SetVisibility _apple8 false false)))
                  (else
                    (Rendering|SetVisibility _apple7 false false)))
                (else
                  (Rendering|SetVisibility _apple6 false false)))
              (else
                (Rendering|SetVisibility _apple5 false false)))
            (else
              (Rendering|SetVisibility _apple4 false false)))
          (else
            (Rendering|SetVisibility (Variables|Default|GetApple3) false false)))
        (else
          (Rendering|SetVisibility (Variables|Default|GetApple2) false false)))
      (else
        (Rendering|SetVisibility (Variables|Default|GetApple1) false false)))))

(fn ConstructionScript)