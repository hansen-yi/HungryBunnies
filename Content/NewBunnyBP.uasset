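; NewBunnyBP is a bunny actor that moves toward the world origin and disappears when it arrives or is caught by the Farmer.
; A timeline started at BeginPlay lerps from the current location to the origin on each update, so movement compounds per frame.
; Tick destroys the bunny after a short delay once it is near the origin.
; Overlapping a Farmer plays the Wink sound at the origin and destroys it immediately.
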(event EventBeginPlay
  (bind _newtrack_0 (Timeline|Timeline Play)
    (:Update
      (Transformation|SetActorLocation (Math|Vector|Lerp(Vector) (Transformation|GetActorLocation) "0, 0, 0" _newtrack_0) false false))))

(event Collision|EventActorBeginOverlap
  (params (OtherActor :type Actor%20Object%20Reference))
  (Utilities|Casting|CastToFarmer OtherActor)
  (Audio|PlaySoundatLocation "/Game/StarterContent/Audio/Wink.Wink" "0, 0, 0" "0, 0, 0" 1.0 1.0 0.0 0 0 0 0)
  (Actor|DestroyActor))

(event EventTick
  (params (DeltaSeconds :type Float%20%28single-precision%29))
  (if (Utilities|Operators|EqualEqual :A (Transformation|GetActorLocation) :ErrorTolerance 0.1)
    (Utilities|FlowControl|Delay 0.5)
    (Actor|DestroyActor)))

(fn ConstructionScript)